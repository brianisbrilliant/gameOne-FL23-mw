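; BP_CameraDoor is a door actor that briefly takes over the first player's view while it opens.
; OpenDoor cubic-blends the camera to this actor, waits, then returns to the passed-in view target in half the blend time.
; The opening itself is only a placeholder print between the blends.
; A separate 5-key event prints a test message, and no input enabling appears in the graph.
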(event `Key|Five`
  (params (Key :type "Key Structure"))
  (:`Pressed`
    (`KismetSystemLibrary.PrintString` "Hello")))

(event `OpenDoor`
  (params (NewViewTarget :type "Actor Object Reference"))
  (bind _blend_time (`self.Blend Time`))
  (`PlayerController.SetViewTargetWithBlend` (`GameplayStatics.GetPlayerController` 0) self _blend_time "VTBlend_Cubic" 0.0 true)
  (`KismetSystemLibrary.Delay` _blend_time)
  (`KismetSystemLibrary.PrintString` "OPENING DOOR NOW")
  (`KismetSystemLibrary.Delay` 2.0)
  (`PlayerController.SetViewTargetWithBlend` (`GameplayStatics.GetPlayerController` 0) NewViewTarget (/ (`self.Blend Time`) 2.0) "VTBlend_Cubic" 0.0 false))

(fn `UserConstructionScript`)