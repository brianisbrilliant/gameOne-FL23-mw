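; Sliding door that opens when the third-person character enters its sphere trigger and closes when the character leaves.
; Overlap begin and end play and reverse a single Timeline, whose float track drives the door mesh's relative Y offset.
; Entering also spawns a sound at the actor's root, which is stopped when the Timeline finishes.
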(event `self.SphereCollision.OnComponentBeginOverlap`
  (params (OverlappedComponent :type "PrimitiveComponent Object Reference") (OtherActor :type "Actor Object Reference") (OtherComp :type "PrimitiveComponent Object Reference") (OtherBodyIndex :type Integer) (bFromSweep :type Boolean) (SweepResult :type "HitResult Structure (by ref)"))
  (cast `/Game/ThirdPerson/Blueprints/BP_ThirdPersonCharacter` OtherActor)
  (bind _returnvalue (`GameplayStatics.SpawnSoundAtLocation` "/Game/Audio/Powerup8_Cue.Powerup8_Cue" (`SceneComponent.K2_GetComponentLocation` (`self.DefaultSceneRoot`)) (struct) 1.0 1.0 0.0 null null))
  (bind (_direction _newtrack_0) (`Timeline|Timeline` :!label _label)
    (:`Update`
      (`SceneComponent.K2_SetRelativeLocation` (`self.Door`) (`KismetMathLibrary.MakeVector` 0.0 (* _newtrack_0 190.0)) false false))
    (:`Finished`
      (`AudioComponent.Stop` _returnvalue))))

(event `self.SphereCollision.OnComponentEndOverlap`
  (params (OverlappedComponent :type "PrimitiveComponent Object Reference") (OtherActor :type "Actor Object Reference") (OtherComp :type "PrimitiveComponent Object Reference") (OtherBodyIndex :type Integer))
  (cast `/Game/ThirdPerson/Blueprints/BP_ThirdPersonCharacter` OtherActor)
  (goto _label :!via `Reverse`))

(fn `UserConstructionScript`)