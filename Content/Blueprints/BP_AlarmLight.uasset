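; Alarm light that flashes its point light red for about five seconds when StartAlarm is called.
; A Sequence starts a timeout that calls StopAlarm, alongside a looping chain of Delays that toggles intensity between zero and its saved value.
; StopAlarm only clears the running flag, so the blink cycle finishes before the color is set to white.
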(event `StartAlarm`
  (bind _pointlight (`self.PointLight`))
  (`|ExecutionSequence`
    (:`then_0`
      (`KismetSystemLibrary.Delay` 5.0) ; wait 5 seconds, then reset alarm
      (if (`self.AlarmIsRunning`)
        (`self.Stop Alarm`)))
    (:`then_1`
      (set `self.AlarmIsRunning` true)
      (set `self.Intensity` (`LightComponentBase.Intensity` _pointlight))
      (`LightComponent.SetLightColor` _pointlight (struct :`R` 1.0 :`B` 0.008842 :`A` 1.0) true)
      (if (`self.AlarmIsRunning`) :!label _label
        (`KismetSystemLibrary.Delay` 0.5)
        (`LightComponent.SetIntensity` _pointlight 0.0)
        (`KismetSystemLibrary.Delay` 0.5)
        (`LightComponent.SetIntensity` _pointlight (`self.Intensity`))
        (goto _label)
        (else
          (`LightComponent.SetLightColor` (`self.PointLight`) (struct :`R` 1.0 :`G` 1.0 :`B` 1.0 :`A` 1.0) true) ; reset light color
        )))))

(event `Stop Alarm`
  (set `self.AlarmIsRunning` false))

(fn `UserConstructionScript`)