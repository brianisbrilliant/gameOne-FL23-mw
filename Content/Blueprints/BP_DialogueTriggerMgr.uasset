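; BP_DialogueTriggerMgr is a dialogue manager that shows lines of text on screen through a W_Dialogue widget.
; It creates the widget and adds it to the viewport on BeginPlay.
; Each PlayNextDialogue call shows the DialogueText entry at the current Index, waits a fixed delay, then advances the Index and clears the text.
; A TODO notes that the duration should depend on string length.
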(event `self.ReceiveBeginPlay`
  (bind _returnvalue (`|CreateWidget` "/Game/WidgetsUI/W_Dialogue.W_Dialogue_C"))
  (`UserWidget.AddToViewport` _returnvalue 0))

(event `PlayNextDialogue`
  (set `/Game/WidgetsUI/W_Dialogue.Dialogue` (`|GetArrayItem` (`self.DialogueText`) (`self.Index`)) (stale `self.ReceiveBeginPlay` _returnvalue))
  (`KismetSystemLibrary.Delay` 2.0) ; TODO: set duration based on # of characters in string
  (`/Engine/EditorBlueprintResources/StandardMacros.IncrementInt` (`self.Index`)
    (:`  `
      (set `/Game/WidgetsUI/W_Dialogue.Dialogue` (`self.EmptyText`) (stale `self.ReceiveBeginPlay` _returnvalue)))))

(fn `UserConstructionScript`)